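; BP_KeyCard is a key card pickup that the player collects by walking into it.
; On overlap with a PlayerCharacter, it inserts true into the KeyCard array at the KeyCardValue index, adds a widget to the viewport and destroys itself.
; Shortly after BeginPlay, it destroys itself if KeyCard index 0 is already true, a fixed index independent of KeyCardValue.
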(event `self.Collision.OnComponentBeginOverlap`
  (params (OverlappedComponent :type "PrimitiveComponent Object Reference") (OtherActor :type "Actor Object Reference") (OtherComp :type "PrimitiveComponent Object Reference") (OtherBodyIndex :type Integer) (bFromSweep :type Boolean) (SweepResult :type "HitResult Structure (by ref)"))
  (cast `/Game/Blueprints/PlayerCharacter` OtherActor)
  (`KismetArrayLibrary.Array_Insert` (`self.KeyCard`) true (`self.KeyCardValue`))
  (bind _returnvalue (`|CreateWidget` null))
  (`UserWidget.AddToViewport` _returnvalue 0)
  (`self.K2_DestroyActor`))

(event `self.ReceiveBeginPlay`
  (`KismetSystemLibrary.Delay` 0.01)
  (cast `/Game/Blueprints/PlayerCharacter` (`GameplayStatics.GetPlayerCharacter` 0))
  (if (`|GetArrayItem` (`self.KeyCard`))
    (`self.K2_DestroyActor`)))

(fn `UserConstructionScript`)